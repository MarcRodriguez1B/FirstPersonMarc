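; Shootable access panel pickup that raises the player's door access level when shot.
; On BeginPlay it caches the player character and tints the panel mesh through a dynamic ID-card material, using the color the door access control component returns for its granted level.
; OnShot sets the player's access level to the granted level, overwriting the current one, then destroys the panel.
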(event `self.ReceiveBeginPlay`
  (bind _asbp_third_person_character (cast `/Game/ThirdPerson/Blueprints/BP_ThirdPersonCharacter` (`GameplayStatics.GetPlayerCharacter` 0)))
  (set `self.Ashe` _asbp_third_person_character)
  (bind _color (`/Game/MyContent/Items/BPC_DoorAccessControl.GetColorDependingOnAccessLevel` (`self.BPC Door Access Control`) (`self.AccessLevelGranted`)))
  (bind _returnvalue (`PrimitiveComponent.CreateDynamicMaterialInstance` (`self.PanelMesh`) 0 "/Game/MyContent/Items/Models/M_IDCard.M_IDCard" "None"))
  (`MaterialInstanceDynamic.SetVectorParameterValue` _returnvalue "Color" _color))

(event `/Game/MyContent/Items/BPI_Shootable.OnShot`
  (params (ShotDirection :type "Vector Structure") (Damage :type "Float (double-precision)"))
  (set `/Game/ThirdPerson/Blueprints/BP_ThirdPersonCharacter.AccessLevel` (`self.AccessLevelGranted`) (`self.Ashe`))
  (`self.K2_DestroyActor`))

(fn `UserConstructionScript`)