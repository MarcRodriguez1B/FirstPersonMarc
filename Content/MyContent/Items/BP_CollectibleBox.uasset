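; BP_CollectibleBox is a collectible item that the player picks up by interacting with it.
; It overrides OnInteract to run the parent logic, increment the Collectible count on the Ashe reference, then destroy itself.
; All other events are disabled stubs, and the construction script only calls its parent.
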(event `/Game/MyContent/Items/BPI_Interactable.OnInteract`
  (bind _ashe (`self.Ashe`))
  (`parent.OnInteract`)
  (bind _result (`/Engine/EditorBlueprintResources/StandardMacros.IncrementInt` (`/Game/ThirdPerson/Blueprints/BP_ThirdPersonCharacter.Collectible` _ashe))
    (:`  `
      (set `/Game/ThirdPerson/Blueprints/BP_ThirdPersonCharacter.Collectible` _result _ashe)
      (`self.K2_DestroyActor`))))

(fn `UserConstructionScript`
  (`parent.UserConstructionScript`))