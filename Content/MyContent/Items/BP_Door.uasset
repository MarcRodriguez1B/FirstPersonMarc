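; BP_Door is a sliding two-panel door that can be locked behind an access level.
; OnInteract compares the player character's AccessLevel to the requirement, then either plays a denied sound or unlocks, turns the frame light green via a dynamic material and opens.
; Once unlocked, any Character's overlap opens or closes it by playing or reversing the DoorAnimation timeline that lerps both panels, with matching sounds.
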(event `self.ReceiveBeginPlay`
  (bind _asbp_third_person_character (cast `/Game/ThirdPerson/Blueprints/BP_ThirdPersonCharacter` (`GameplayStatics.GetPlayerCharacter` 0)))
  (set `self.Ashe` _asbp_third_person_character))

(event `/Game/MyContent/Items/BPI_Interactable.OnInteract`
  (bind _returnvalue (`self.K2_GetActorLocation`))
  (if (`self.Locked`)
    (if (>= (`/Game/ThirdPerson/Blueprints/BP_ThirdPersonCharacter.AccessLevel` (`self.Ashe`)) (`self.AccessLevelRequired`))
      (`GameplayStatics.PlaySoundAtLocation` "/Game/MyContent/Items/SFX/Door/SC_Door_AccesGranted.SC_Door_AccesGranted" _returnvalue (struct) 1.0 1.0 0.0 null null null null)
      (set `self.Locked` false)
      (bind _returnvalue_2 (`PrimitiveComponent.CreateDynamicMaterialInstance` (`self.SM_Door_Frame`) 1 "/Game/MyContent/Items/Models/M_DoorLight.M_DoorLight" "None"))
      (`MaterialInstanceDynamic.SetVectorParameterValue` _returnvalue_2 "Color" (struct :`R` 0.045561 :`G` 1.0 :`A` 1.0))
      (`GameplayStatics.PlaySoundAtLocation` "/Game/MyContent/Items/SFX/Door/SC_Door_Open.SC_Door_Open" (`self.K2_GetActorLocation`) (struct) 1.0 1.0 0.0 null null null null :!label _label)
      (bind (_direction _alpha) (`Timeline|Door Animation` :!label _label_2)
        (:`Update`
          (`SceneComponent.K2_SetRelativeLocation` (`self.SM_Door_Panel_R`) (`KismetMathLibrary.VLerp` (0.0 0.0 0.0) (100.0 0.0 0.0) _alpha) false false)
          (`SceneComponent.K2_SetRelativeLocation` (`self.SM_Door_Panel_L`) (`KismetMathLibrary.VLerp` (0.0 0.0 0.0) (-80.0 0.0 0.0) _alpha) false false)))
      (else
        (`GameplayStatics.PlaySoundAtLocation` "/Game/MyContent/Items/SFX/Door/SC_Door_AccessDenied.SC_Door_AccessDenied" _returnvalue (struct) 1.0 1.0 0.0 null null null null)))))

(event `self.ReceiveActorBeginOverlap`
  (params (OtherActor :type "Actor Object Reference"))
  (bind _ascharacter (cast `Character` OtherActor))
  (`/Engine/EditorBlueprintResources/StandardMacros.IsValid` _ascharacter
    (:`Is Valid`
      (if (not (`self.Locked`))
        (goto _label)))))

(event `self.ReceiveActorEndOverlap`
  (params (OtherActor :type "Actor Object Reference"))
  (bind _ascharacter (cast `Character` OtherActor))
  (`/Engine/EditorBlueprintResources/StandardMacros.IsValid` _ascharacter
    (:`Is Valid`
      (if (not (`self.Locked`))
        (`GameplayStatics.PlaySoundAtLocation` "/Game/MyContent/Items/SFX/Door/SC_Door_Close.SC_Door_Close" (`self.K2_GetActorLocation`) (struct) 1.0 1.0 0.0 null null null null)
        (goto _label_2 :!via `Reverse`)))))

(fn `UserConstructionScript`)