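; BP_ExplosiveBarrel is a shootable barrel that deals area damage once its health runs out.
; OnShot feeds damage into a health macro, which clamps the result and signals when it reaches zero.
; At zero, the barrel removes its mesh and briefly enables the sphere collision, disabled since BeginPlay, before destroying itself.
; Actors beginning overlap with the sphere receive a fixed negative damage message if they implement BPI_Damageable.
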(event `self.ReceiveBeginPlay`
  (`PrimitiveComponent.SetCollisionEnabled` (`self.SphereCollision`) "NoCollision"))

(event `/Game/MyContent/Items/BPI_Shootable.OnShot`
  (params (ShotDirection :type "Vector Structure") (Damage :type "Float (double-precision)"))
  (`self.Barrel Health Macro` Damage
    (:`True`
      (`PrimitiveComponent.SetCollisionEnabled` (`self.SphereCollision`) "QueryAndPhysics")
      (`ActorComponent.K2_DestroyComponent` (`self.BarrelMesh`))
      (`KismetSystemLibrary.Delay` 0.2)
      (`self.K2_DestroyActor`))))

(event `self.SphereCollision.OnComponentBeginOverlap`
  (params (OverlappedComponent :type "PrimitiveComponent Object Reference") (OtherActor :type "Actor Object Reference") (OtherComp :type "PrimitiveComponent Object Reference") (OtherBodyIndex :type Integer) (bFromSweep :type Boolean) (SweepResult :type "HitResult Structure (by ref)"))
  (if (`KismetSystemLibrary.DoesImplementInterface` OtherActor "/Game/MyContent/Items/BPI_Damageable.BPI_Damageable_C")
    (message `/Game/MyContent/Items/BPI_Damageable.OnDamaged` OtherActor -60.0)))

(fn `UserConstructionScript`)