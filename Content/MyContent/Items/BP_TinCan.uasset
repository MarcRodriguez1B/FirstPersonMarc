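; BP_TinCan is an interactable tin can item that gets knocked away when the player interacts with it.
; OnInteract runs the parent logic, then applies an impulse to the mesh along the horizontal components of Ashe's follow camera forward vector, with a fixed upward kick.
; The other events are disabled stubs, and the construction script only calls its parent.
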(event `/Game/MyContent/Items/BPI_Interactable.OnInteract`
  (bind (_returnvalue_x _returnvalue_y) (`KismetMathLibrary.BreakVector` (* (`SceneComponent.GetForwardVector` (`/Game/ThirdPerson/Blueprints/BP_ThirdPersonCharacter.FollowCamera` (`self.Ashe`))) 5000.0)))
  (`parent.OnInteract`)
  (`PrimitiveComponent.AddImpulse` (`self.Mesh`) (`KismetMathLibrary.MakeVector` _returnvalue_x _returnvalue_y 5000.0) "None" false))

(fn `UserConstructionScript`
  (`parent.UserConstructionScript`))