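; Velkoz enemy character that patrols, roams or guards around a patrol point, then chases and fires projectiles at the player (Ashe).
; Event-driven AIMoveTo logic replaces a behavior tree: sight or damage triggers an alert, Cry also grants aggro, and chase alternates with cooldown-gated attacks.
; A retriggerable delay after sightings drops aggro and resumes the base behavior.
; A health macro routes hits to alert or to a montage-and-dissolve death.
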(event `self.ReceiveBeginPlay`
  (`self.Launch Base Behavior`)
  (bind _asbp_third_person_character (cast `/Game/ThirdPerson/Blueprints/BP_ThirdPersonCharacter` (`GameplayStatics.GetPlayerCharacter` 0)))
  (set `self.Ashe` _asbp_third_person_character))

(event `Event OnShot`
  (params (`Shot Direction` :type "Vector Structure") (Damage :type "Float (double-precision)"))
  ;[0.1035 0.02146 0.15 0.5] Damage to Self
  (`self.Health Manager Velkoz Macro` Damage
    (:`Is Dead`
      (`self.Death`))
    (:`Is Alive`
      (if (not (`self.HasAggro`))
        (`/Engine/EditorBlueprintResources/StandardMacros.DoOnce` false
          (:`Completed`
            (`self.Behavior Alert`)))))))

(event `Event OnDamaged`
  (params (Damage :type "Float (double-precision)"))
  ;[0.1035 0.02146 0.15 0.5] Damage to Self
  (`self.Health Manager Velkoz Macro` Damage
    (:`Is Dead`
      (`self.Death`))
    (:`Is Alive`
      (if (not (`self.HasAggro`))
        (`self.Behavior Alert`)))))

(event `Launch Base Behavior`
  ;[0.15 0.054 0 0.5] Base Behaviors
  (switch `/Game/MyContent/Character/Enemy/Enum_EnemyStates` (`self.BaseBahavior`)
    (:`NewEnumerator0`
      (`self.Behavior Patrol`))
    (:`NewEnumerator1`
      (`self.Behavior Roam`))
    (:`NewEnumerator2`
      (`self.Behavior Guard`))))

(event `Behavior Guard`
  ;[0.15 0.054 0 0.5] Base Behaviors
  (`|AIMoveTo` self (0.0 0.0 0.0) (`self.PatrolPoint`) 0.0
    (:`OnSuccess`
      (set `self.Guard_InitialRotation` (`self.K2_GetActorRotation`))
      (set `self.Guard_EndRotation` (`self.K2_GetActorRotation` (`self.PatrolPoint`)))
      (bind (_direction _alpha) (`Timeline|Timeline`)
        (:`Update`
          (`self.K2_SetActorRotation` (`KismetMathLibrary.RLerp` (`self.Guard_InitialRotation`) (`self.Guard_EndRotation`) _alpha)))
        (:`Finished`
          (`self.K2_DestroyActor`))))))

(event `Death`
  ;[0.1035 0.02146 0.15 0.5] Damage to Self
  (`/Engine/EditorBlueprintResources/StandardMacros.DoOnce` false
    (:`Completed`
      (`CharacterMovementComponent.SetMovementMode` (`self.CharacterMovement`) "MOVE_None" 0)
      (bind _returnvalue (`self.PlayAnimMontage` "/Game/MyContent/Character/Enemy/Velkoz/Assets/Anim/AM_Velkoz_Death.AM_Velkoz_Death"))
      (bind (_direction _dissolve) (`Timeline|Dissolve` :!via `PlayFromStart`)
        (:`Update`
          (`MeshComponent.SetScalarParameterValueOnMaterials` (`self.Mesh`) "Dissolve" (`KismetMathLibrary.Lerp` -1.0 1.0 _dissolve)))
        (:`Finished`
          (`KismetSystemLibrary.Delay` _returnvalue)
          (`self.K2_DestroyActor`))))))

(event `Behavior Patrol`
  ;[0.15 0.054 0 0.5] Base Behaviors
  (if (not (`self.HasAggro`))
    (`|AIMoveTo` self (0.0 0.0 0.0) (`self.PatrolPoint`)
      (:`OnSuccess`
        (`KismetSystemLibrary.Delay` (`KismetMathLibrary.RandomFloatInRange` 2.0 5.0))
        (set `self.PatrolPoint` (`/Game/MyContent/Character/Enemy/BP_PatrolPoint.NextPatrolPoint` (`self.PatrolPoint`)))
        (`self.Behavior Patrol`)))))

(event `Behavior Attack`
  ;[0.15 3e-06 0.000645 0.5] Attack
  (`/Engine/EditorBlueprintResources/StandardMacros.DoOnce` false :!label _label
    (:`Completed`
      (`self.PlayAnimMontage` "/Game/MyContent/Character/Enemy/Velkoz/Assets/Anim/AM_Velkoz_Attack.AM_Velkoz_Attack")
      (`self.Projectile`)
      (`KismetSystemLibrary.Delay` (`self.AttackCooldown`))
      (`self.Reset Attack`)
      (`self.Behavior Chase`))))

(event `Reset Attack`
  ;[0.15 3e-06 0.000645 0.5] Attack
  (goto _label :!via `Reset`))

(event `Projectile`
  ;[0.15 3e-06 0.000645 0.5] Attack
  (`self.Redirect Attack`)
  (`|SpawnActorFromClass` "/Game/MyContent/Character/Enemy/Velkoz/BP_Projectile_Velkoz.BP_Projectile_Velkoz_C" (`KismetMathLibrary.MakeTransform` (`SceneComponent.K2_GetComponentLocation` (`self.ProjectileSpawn`)) (`KismetMathLibrary.Conv_VectorToRotator` (`SceneComponent.GetForwardVector` (`self.CapsuleComponent`)))) "Undefined" "MultiplyWithRoot" null null)
  (`GameplayStatics.PlaySoundAtLocation` "/Game/MyContent/Character/Ashe/Weapon/SFX/SC_VelkozBasic.SC_VelkozBasic" (0.0 0.0 0.0) (struct) 1.0 1.0 0.0 null null null null))

(event `Redirect Attack`
  ;[0.15 3e-06 0.000645 0.5] Attack
  (`self.K2_SetActorRotation` (`KismetMathLibrary.FindLookAtRotation` (`self.K2_GetActorLocation`) (`self.K2_GetActorLocation` (`self.Ashe`)))))

(event `Behavior Roam`
  ;[0.15 0.054 0 0.5] Base Behaviors
  (if (not (`self.HasAggro`))
    (bind _randomlocation (`NavigationSystemV1.K2_GetRandomLocationInNavigableRadius` (`self.K2_GetActorLocation` (`self.PatrolPoint`)) (`self.Roam Radius`) null null))
    (if (> (`KismetMathLibrary.Vector_Distance` _randomlocation (`self.K2_GetActorLocation`)) 0.0)
      (`|AIMoveTo` self _randomlocation null
        (:`then`
          (`KismetSystemLibrary.Delay` (`KismetMathLibrary.RandomFloatInRange` 2.0 5.0))))
      (else
        (`self.Behavior Roam`)))))

(event `self.PawnSensing.OnSeePawn`
  (params (Pawn :type "Pawn Object Reference"))
  ;[0.02242 0.15 0.1256 0.5] Sensing and Chasing
  (if (== Pawn (`self.Ashe`))
    (`self.Try Not See Pawn`)
    (if (not (`self.HasAggro`))
      (`self.Behavior Alert`))))

(event `Behavior Stop`
  ;[0.02242 0.15 0.1256 0.5] Sensing and Chasing
  (`|AIMoveTo` self (0.0 0.0 0.0) self))

(event `Try Not See Pawn`
  ;[0.02242 0.15 0.1256 0.5] Sensing and Chasing
  (`KismetSystemLibrary.RetriggerableDelay` 10.0)
  (`self.Behavior Stop`)
  (set `self.HasAggro` false)
  (`self.Reset Alert`)
  (`KismetSystemLibrary.Delay` 2.0)
  (if (not (`self.HasAggro`))
    (`self.Launch Base Behavior`)))

(event `Cry`
  ;[0.02242 0.15 0.1256 0.5] Sensing and Chasing
  (if (not (`self.HasAggro`))
    (set `self.HasAggro` true)
    (`self.Behavior Stop`)
    (bind _returnvalue (`self.PlayAnimMontage` "/Game/MyContent/Character/Enemy/Velkoz/Assets/Anim/AM_Velkoz_Cry.AM_Velkoz_Cry"))
    (`KismetSystemLibrary.Delay` _returnvalue)
    (`self.Behavior Chase`)))

(event `Behavior Chase`
  ;[0.02242 0.15 0.1256 0.5] Sensing and Chasing
  (`|AIMoveTo` self (0.0 0.0 0.0) (`self.Ashe`) (`self.AttackDistance`)
    (:`then`
      (if (> (`self.Health`) 0.0)
        (`self.Behavior Attack`)))))

(event `Behavior Alert`
  ;[0.02242 0.15 0.1256 0.5] Sensing and Chasing
  (`/Engine/EditorBlueprintResources/StandardMacros.DoOnce` false :!label _label_2
    (:`Completed`
      (set `self.HasAggro` true)
      (`self.Behavior Stop`)
      (`|SpawnActorFromClass` "/Game/MyContent/Character/Enemy/BP_EnemyAlert.BP_EnemyAlert_C" (`KismetMathLibrary.MakeTransform` (`self.K2_GetActorLocation`)) "Undefined" "MultiplyWithRoot" null null)
      (bind _returnvalue (`self.PlayAnimMontage` "/Game/MyContent/Character/Enemy/Velkoz/Assets/Anim/AM_Velkoz_AreaAlert.AM_Velkoz_AreaAlert"))
      (`KismetSystemLibrary.Delay` _returnvalue)
      (`self.Behavior Chase`))))

(event `Reset Alert`
  ;[0.02242 0.15 0.1256 0.5] Sensing and Chasing
  (goto _label_2 :!via `Reset`))

(event `/Game/MyContent/Items/BPI_Shootable.OnShot`
  (params (ShotDirection :type "Vector Structure") (Damage :type "Float (double-precision)"))
  (`self.Health Manager Velkoz Macro` Damage
    (:`Is Dead`
      (`self.Death`))
    (:`Is Alive`
      (if (not (`self.HasAggro`))
        (`self.Behavior Alert`)))))

(event `/Game/MyContent/Items/BPI_Damageable.OnDamaged`
  (params (Damage :type "Float (double-precision)"))
  (`self.Health Manager Velkoz Macro` Damage
    (:`Is Dead`
      (`self.Death`))
    (:`Is Alive`
      (if (not (`self.HasAggro`))
        (`self.Behavior Alert`)))))

(fn `UserConstructionScript`)