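; Fiddlesticks enemy character that patrols linked points, roams or guards, and fights the player (Ashe).
; AIMoveTo-driven events form the behaviors; surviving a shot triggers a cry, then a chase looping into close or mid-range montage attacks.
; Sightings set aggro before checking it, so the alert branch looks unreachable; a retriggerable delay later restores base behavior.
; Guard destroys the actor after rotating, and death requires health exactly zero, without clamping.
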(event `self.ReceiveBeginPlay`
  (`self.LaunchBaseBehavior`)
  (bind _asbp_third_person_character (cast `/Game/ThirdPerson/Blueprints/BP_ThirdPersonCharacter` (`GameplayStatics.GetPlayerCharacter` 0)))
  (set `self.Ashe` _asbp_third_person_character))

(event `LaunchBaseBehavior`
  (switch `/Game/MyContent/Character/Enemy/Enum_EnemyStates` (`self.BaseBehavior`)
    (:`NewEnumerator0`
      (`self.BehaviorPatrol`))
    (:`NewEnumerator1`
      (`self.BehaviorRoam`))
    (:`NewEnumerator2`
      (`self.BehaviorGuard`))))

(event `BehaviorGuard`
  (`|AIMoveTo` self (0.0 0.0 0.0) (`self.PatrolPoint`) 0.0
    (:`OnSuccess`
      (set `self.Guard_InitialRotation` (`self.K2_GetActorRotation`))
      (set `self.Guard_EndRotation` (`self.K2_GetActorRotation` (`self.PatrolPoint`)))
      (bind (_direction _alpha) (`Timeline|GuardRotationAnimation`)
        (:`Update`
          (`self.K2_SetActorRotation` (`KismetMathLibrary.RLerp` (`self.Guard_InitialRotation`) (`self.Guard_EndRotation`) _alpha)))
        (:`Finished`
          (`self.K2_DestroyActor`))))))

(event `BehaviorPatrol`
  (if (not (`self.HasAggro`))
    (`|AIMoveTo` self (0.0 0.0 0.0) (`self.PatrolPoint`)
      (:`OnSuccess`
        (`KismetSystemLibrary.Delay` (`KismetMathLibrary.RandomFloatInRange` 2.0 5.0))
        (set `self.PatrolPoint` (`/Game/MyContent/Character/Enemy/BP_PatrolPoint.NextPatrolPoint` (`self.PatrolPoint`)))
        (`self.LaunchBaseBehavior`)))))

(event `BehaviorRoam`
  (if (not (`self.HasAggro`))
    (bind _randomlocation (`NavigationSystemV1.K2_GetRandomLocationInNavigableRadius` (`self.K2_GetActorLocation` (`self.PatrolPoint`)) (`self.Roam Radius`) null null))
    (if (> (`KismetMathLibrary.Vector_Distance` _randomlocation (`self.K2_GetActorLocation`)) 0.0)
      (`|AIMoveTo` self _randomlocation null
        (:`then`
          (`KismetSystemLibrary.Delay` (`KismetMathLibrary.RandomFloatInRange` 2.0 5.0))
          (`self.BehaviorRoam`)))
      (else
        (`self.BehaviorRoam`)))))

(event `/Game/MyContent/Items/BPI_Shootable.OnShot`
  (params (ShotDirection :type "Vector Structure") (Damage :type "Float (double-precision)"))
  (`self.HealthManager` Damage
    (:`Is Dead`
      (`self.Death`))
    (:`Is Alive`
      (if (not (`self.HasAggro`))
        (`self.Cry`)))))

(event `Death`
  (`/Engine/EditorBlueprintResources/StandardMacros.DoOnce` false
    (:`Completed`
      (`CharacterMovementComponent.SetMovementMode` (`self.CharacterMovement`) "MOVE_None" 0)
      (bind _returnvalue (`self.PlayAnimMontage` (`KismetArrayLibrary.Array_Random` (`self.Anim_Death`))))
      (`KismetSystemLibrary.Delay` _returnvalue)
      (`self.K2_DestroyActor`))))

(event `BehaviorAlert`
  (`/Engine/EditorBlueprintResources/StandardMacros.DoOnce` false :!label _label
    (:`Completed`
      (set `self.HasAggro` true)
      (`self.BehaviorStop`)
      (`|SpawnActorFromClass` "/Game/MyContent/Character/Enemy/BP_EnemyAlert.BP_EnemyAlert_C" (`KismetMathLibrary.MakeTransform` (`self.K2_GetActorLocation`)) "Undefined" "MultiplyWithRoot" null null)
      (bind _returnvalue (`self.PlayAnimMontage` "/Game/MyContent/Character/Enemy/Fiddlesticks/AM_FiddlesticksAreaAlert.AM_FiddlesticksAreaAlert"))
      (`KismetSystemLibrary.Delay` _returnvalue)
      (`self.BehaviorChase`))))

(event `ResetAlert`
  (goto _label :!via `Reset`))

(event `self.PawnSensing.OnSeePawn`
  (params (Pawn :type "Pawn Object Reference"))
  (if (== Pawn (`self.Ashe`))
    (set `self.HasAggro` true)
    (`self.TryNotSeePawn`)
    (if (not (`self.HasAggro`))
      (`self.BehaviorAlert`))))

(event `Cry`
  (if (not (`self.HasAggro`))
    (set `self.HasAggro` true)
    (`self.BehaviorStop`)
    (bind _returnvalue (`self.PlayAnimMontage` "/Game/MyContent/Character/Enemy/Fiddlesticks/AM_Fiddlesticks_Cry.AM_Fiddlesticks_Cry"))
    (`KismetSystemLibrary.Delay` _returnvalue)
    (`self.BehaviorChase`)))

(event `TryNotSeePawn`
  (`KismetSystemLibrary.RetriggerableDelay` 5.0)
  (`self.BehaviorStop`)
  (set `self.HasAggro` false)
  (`self.ResetAlert`)
  (`KismetSystemLibrary.Delay` 2.0)
  (if (not (`self.HasAggro`))
    (`self.LaunchBaseBehavior`)))

(event `BehaviorStop`
  (`|AIMoveTo` self (0.0 0.0 0.0) self))

(event `BehaviorChase`
  (`|AIMoveTo` self (0.0 0.0 0.0) (`self.Ashe`) (`self.Attack Distance`)
    (:`OnSuccess`
      (`self.BehaviorAttack`))))

(event `BehaviorAttack`
  (`/Engine/EditorBlueprintResources/StandardMacros.DoOnce` false :!label _label_2
    (:`Completed`
      (if (<= (`KismetMathLibrary.Vector_Distance` (`self.K2_GetActorLocation`) (`self.K2_GetActorLocation` (`self.Ashe`))) 200.0)
        (`/Engine/EditorBlueprintResources/StandardMacros.FlipFlop`
          (:`A`
            (`self.PlayAnimMontage` "/Game/MyContent/Character/Enemy/Fiddlesticks/AM_Fiddlesticks_CloseAttack_01.AM_Fiddlesticks_CloseAttack_01")
            (`KismetSystemLibrary.Delay` 0.85))
          (:`B`
            (`self.PlayAnimMontage` "/Game/MyContent/Character/Enemy/Fiddlesticks/Animations/AM_Fiddlesticks_CloseAttack_02.AM_Fiddlesticks_CloseAttack_02")
            (`KismetSystemLibrary.Delay` 0.85)))
        (else
          (`self.PlayAnimMontage` "/Game/MyContent/Character/Enemy/Fiddlesticks/Animations/AM_Fiddlesticks_MidAttack.AM_Fiddlesticks_MidAttack")
          (`KismetSystemLibrary.Delay` 0.8)))
      (`self.ResetAttack`)
      (`self.BehaviorChase`))))

(event `ResetAttack`
  (goto _label_2 :!via `Reset`))

(fn `UserConstructionScript`)