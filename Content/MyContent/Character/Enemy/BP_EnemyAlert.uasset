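; BP_EnemyAlert is an expanding alert zone that makes enemies it reaches cry out.
; On BeginPlay, a timeline scaled by Duration grows the sphere collision from a small radius to a wide one, updating overlaps each step.
; Actors that begin overlapping are class-checked, cast to BP_Enemy, and have their Cry function called.
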(event `self.ReceiveBeginPlay`
  (`TimelineComponent.SetPlayRate` (`self.AlertExpansion`) (/ 1.0 (`self.Duration`)))
  (bind (_direction _alpha) (`Timeline|AlertExpansion`)
    (:`Update`
      (`SphereComponent.SetSphereRadius` (`self.Sphere`) (`KismetMathLibrary.Lerp` 32.0 2000.0 _alpha) true))))

(event `self.ReceiveActorBeginOverlap`
  (params (OtherActor :type "Actor Object Reference"))
  (if (== (`GameplayStatics.GetObjectClass` OtherActor) null)
    (bind _asbp_enemy (cast `/Game/MyContent/Character/Enemy/BP_Enemy` OtherActor))
    (`/Game/MyContent/Character/Enemy/BP_Enemy.Cry` _asbp_enemy)))

(fn `UserConstructionScript`)